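; BP_Node_Editor is an actor-style Blueprint that opens a node editor UI at game start.
; On BeginPlay it creates UI_Node_Editor, stores it and adds it to the viewport.
; It then builds two UI_Nodes windows, each wrapping a separate child widget with its own title, position and look, and passes them the editor reference before placing them on its canvas.
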(event EventBeginPlay
  (bind _returnvalue (UserInterface|CreateWidget "/WindowSystem/Nodes/Widgets/UI_Node_Editor.UI_Node_Editor_C"))
  (bind _output_get (Variables|Default|SetREF_Node_Editor _returnvalue))
  (UserInterface|Viewport|AddtoViewport _output_get 0)
  (Utilities|FlowControl|Sequence
    (:then_0
      (bind _returnvalue_2 (UserInterface|CreateWidget "/WindowSystem/Debug/Widgets/UI_Window.UI_Window_C"))
      (bind _returnvalue_3 (UserInterface|CreateWidget "/WindowSystem/Nodes/Widgets/UI_Nodes.UI_Nodes_C" 0 _returnvalue_2 "Node1" "(X=512.000000,Y=512.000000)" "(R=0.250000,G=0.250000,B=0.250000,A=1.000000)" "(R=1.000000,G=1.000000,B=1.000000,A=1.000000)" "(X=100.000000,Y=100.000000)" (Variables|Default|GetREF_Node_Editor)))
      (Class|CanvasPanel|AddChildtoCanvas (Variables|/WindowSystem/Nodes/Widgets/UI_Node_Editor.UI_Node_Editor_C|GetCANVAS (Variables|Default|GetREF_Node_Editor)) _returnvalue_3))
    (:then_1
      (bind _returnvalue_4 (UserInterface|CreateWidget "/WindowSystem/Debug/Widgets/UI_Child_Window.UI_Child_Window_C"))
      (bind _returnvalue_5 (UserInterface|CreateWidget "/WindowSystem/Nodes/Widgets/UI_Nodes.UI_Nodes_C" 0 _returnvalue_4 "Node2" "(X=512.000000,Y=512.000000)" "(R=1.000000,G=0.000000,B=0.000000,A=1.000000)" "(R=1.000000,G=1.000000,B=1.000000,A=1.000000)" "(X=600.000000,Y=450.000000)" (Variables|Default|GetREF_Node_Editor)))
      (Class|CanvasPanel|AddChildtoCanvas (Variables|/WindowSystem/Nodes/Widgets/UI_Node_Editor.UI_Node_Editor_C|GetCANVAS (Variables|Default|GetREF_Node_Editor)) _returnvalue_5))))

(fn ConstructionScript)